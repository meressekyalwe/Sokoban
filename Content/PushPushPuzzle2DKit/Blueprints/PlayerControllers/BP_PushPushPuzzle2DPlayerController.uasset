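; Player controller for the PushPushPuzzle 2D kit that owns the HUD and switches between gameplay and menu input.
; On BeginPlay it creates the BP_HUD widget, adds it to the viewport and sets game-only input.
; The Pause Game input shows the pause menu, pauses, and enables the cursor with UI-only input, which UnpauseGame reverses.
; ShowLevelCompleteOverview forwards level results to the HUD and switches to UI input.
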(event EventBeginPlay
  ;[1 1 1] Create HUD Widget and add to viewport
  (bind _returnvalue (UserInterface|CreateWidget "/Game/PushPushPuzzle2DKit/Blueprints/Widgets/BP_HUD.BP_HUD_C"))
  (bind _output_get (Variables|Default|SetHUD _returnvalue))
  (UserInterface|Viewport|AddtoViewport _output_get 0)
  ;[1 1 1] Set the input to game only
  (Input|SetInputModeGameOnly self))

(event Input|ActionEvents|InputActionPauseGame
  (params (Key :type Key%20Structure))
  (:Pressed
    (CallFunction|PauseGame)))

(fn ConstructionScript)

(fn PauseGame
  ;[1 1 1] Show the pause menu
  (bind _hud (Variables|Default|GetHUD)
    (:then
      (Default|ShowPauseMenu _hud)
      ;[1 1 1] Set game to paused, show mouse cursor and set the input to UI only
      (Game|SetGamePaused true)
      (Variables|Default|SetbShowMouseCursor true)
      (Input|SetInputModeUIOnly self 0 "DoNotLock"))
    (:else)))

(fn UnpauseGame
  ;[1 1 1] Unpause the game
  (Game|SetGamePaused false)
  ;[1 1 1] Hide mouse cursor and set input to game only
  (Variables|Default|SetbShowMouseCursor false)
  (Input|SetInputModeGameOnly self))

(fn ShowLevelCompleteOverview
  (params (Moves :type Integer) (Time :type Float%20%28single-precision%29) (Coins :type Integer) (MovesImproved :type Boolean) (TimeImproved :type Boolean) (CoinsImproved :type Boolean) (NextLevelAvailable :type Boolean))
  ;[1 1 1] Update the HUD
  (Default|ShowLevelCompleteMenu (Variables|Default|GetHUD) Moves Time Coins MovesImproved TimeImproved CoinsImproved NextLevelAvailable)
  ;[1 1 1] Show mouse cursor and set input UI only
  (Variables|Default|SetbShowMouseCursor true)
  (Input|SetInputModeUIOnly self 0 "DoNotLock"))