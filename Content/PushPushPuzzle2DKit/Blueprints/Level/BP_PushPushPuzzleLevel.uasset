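; Level actor for a 2D push puzzle that turns a painted tile map into playable boxes, goals, coins and a player start.
; Reset hides the player, parses tile user data strings into type and color, clears the marker layer, spawns actors and positions the player.
; Goals register with the game mode, boxes and goals receive their color, and fixed world Y values set sprite draw order.
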(fn ConstructionScript)

(fn AnalyzeTileMap
  ;[1 1 1] Loop through all the tiles
  (bind (_mapwidth _mapheight _numlayers) (Class|PaperTileMapComponent|GetMapSize (Variables|Default|GetTileMap)))
  (for _index (range 0 _numlayers)
    (for _index_2 (range 0 _mapheight)
      (for _index_3 (range 0 _mapwidth)
        ;[1 1 1] Analyze the tile user data to determine the type (player start, box or goal) and color
        (LocalVariables|SetTileLocation (Utilities|Struct|MakeSTR_TileMapLocation _index_3 _index_2 _index))
        (if (.ReturnValue (Utilities|String|Split (CallFunction|GetTileUserDataString (LocalVariables|GetTileLocation)) "_"))
          (switch string (.LeftS (Utilities|String|Split (CallFunction|GetTileUserDataString (LocalVariables|GetTileLocation)) "_"))
            (:PlayerStart
              ;[1 1 1] Save the player start position, use Y = 5 to always draw player at top
              (Variables|Spawning|SetPlayerStartLocation (TileMap|TileMaptoWorld (LocalVariables|GetTileLocation) 5.0)))
            (:Box
              ;[1 1 1] Add the box spawn location to the array
              (Utilities|Array|AddUnique (Variables|Spawning|GetBoxSpawnLocations) (Utilities|Struct|MakeSTR_SpawnInformation (LocalVariables|GetTileLocation) (Helper|StringtoColor (.RightS (Utilities|String|Split (CallFunction|GetTileUserDataString (LocalVariables|GetTileLocation)) "_"))))))
            (:Goal
              ;[1 1 1] Add the goal spawn location to the array
              (Utilities|Array|AddUnique (Variables|Spawning|GetGoalSpawnLocations) (Utilities|Struct|MakeSTR_SpawnInformation (LocalVariables|GetTileLocation) (Helper|StringtoColor (.RightS (Utilities|String|Split (CallFunction|GetTileUserDataString (LocalVariables|GetTileLocation)) "_"))))))
            (:Coin
              ;[1 1 1] Add the coin spawn location to the array, color is irrelevant
              (Utilities|Array|AddUnique (Variables|Spawning|GetCoinSpawnLocations) (Utilities|Struct|MakeSTR_SpawnInformation (LocalVariables|GetTileLocation) "NewEnumerator0")))))))))

(fn TileMaptoWorld
  (params (TileMapLocation :type STR%20Tile%20Map%20Location%20Structure) (Y-coordinate :type Float%20%28single-precision%29))
  (bind _tilemap (Variables|Default|GetTileMap))
  (bind _tilemap_2 (Variables|/Script/Paper2D.PaperTileMapComponent|GetTileMap _tilemap))
  ;[1 1 1] Negate the y location
  (bind _result (Utilities|NegateInt (.y TileMapLocation))
    (:%20%20
      (return (+ (Transformation|GetWorldLocation _tilemap) (Math|Vector|MakeVector (Math|Conversions|ToFloat(Integer) (* (.x TileMapLocation) (Variables|/Script/Paper2D.PaperTileMap|GetTileWidth _tilemap_2))) Y-coordinate (Math|Conversions|ToFloat(Integer) (* _result (Variables|/Script/Paper2D.PaperTileMap|GetTileHeight _tilemap_2)))))))))

(fn SpawnActorsfromTileMapLocations
  (params (SpawnInformations :type Array%20of%20STR%20Spawn%20Information%20Structures) (ClassToSpawn :type Actor%20Class%20Reference) (Y-coordinate :type Float%20%28single-precision%29))
  ;[1 1 1] Loop through the spawn info
  (for _array_element SpawnInformations
    ;[1 1 1] Convert location to world location and spawn actor
    (LocalVariables|SetColor (.color _array_element))
    (bind _returnvalue (Game|SpawnActorfromClass ClassToSpawn (Math|Transform|MakeTransform (TileMap|TileMaptoWorld (.tilemaplocation _array_element) Y-coordinate) "0, 0, 0" "1,1,1") "Undefined" 0 0))
    ;[1 1 1] Add a goal to the goals array of the game mode and update color
    (bind _asbp_goal (Utilities|Casting|CastToBP_Goal _returnvalue)
      (:then
        (Utilities|Array|AddUnique (Variables|/Game/PushPushPuzzle2DKit/Blueprints/Game/BP_PushPushPuzzle2DGameMode.BP_PushPushPuzzle2DGameMode_C|GetGoals (Variables|Default|GetGameMode)) _asbp_goal)
        (Default|UpdateColor _asbp_goal (LocalVariables|GetColor)))
      (:CastFailed
        ;[1 1 1] For boxes, just update the color
        (bind _asbp_box (Utilities|Casting|CastToBP_Box _returnvalue))
        (Default|UpdateColor _asbp_box (LocalVariables|GetColor))))))

(fn ClearGameTileMapLayer
  (bind _tilemap (Variables|Default|GetTileMap))
  ;[1 1 1] Make the tile map editable
  (Class|PaperTileMapComponent|MakeTileMapEditable _tilemap)
  ;[1 1 1] Loop trough all positions of the first layer (which has the spawn data)
  (bind (_mapwidth _mapheight) (Class|PaperTileMapComponent|GetMapSize _tilemap))
  (for _index (range 0 _mapheight)
    (for _index_2 (range 0 _mapwidth)
      ;[1 1 1] Clear the tile
      (Class|PaperTileMapComponent|SetTile (Variables|Default|GetTileMap) _index_2 _index 0 (Utilities|Struct|MakePaperTileInfo -1 0 false false false)))))

(fn SpawnGameActors
  ;[1 1 1] Spawn all boxes, Y = 4 to draw over the goals
  (Spawning|SpawnActorsfromTileMapLocations (Variables|Spawning|GetBoxSpawnLocations) "/Game/PushPushPuzzle2DKit/Blueprints/Objects/BP_Box.BP_Box_C" 4.0)
  ;[1 1 1] Spawn all goals, Y = 3 to draw under the boxes
  (Spawning|SpawnActorsfromTileMapLocations (Variables|Spawning|GetGoalSpawnLocations) "/Game/PushPushPuzzle2DKit/Blueprints/Objects/BP_Goal.BP_Goal_C" 3.0)
  ;[1 1 1] Spawn all coins
  (Spawning|SpawnActorsfromTileMapLocations (Variables|Spawning|GetCoinSpawnLocations) "/Game/PushPushPuzzle2DKit/Blueprints/Objects/BP_Coin.BP_Coin_C" 3.0))

(fn PositionPlayer
  (params (Position :type Vector))
  (bind _returnvalue (Game|Player|GetPlayerPawn 0))
  (Utilities|IsValid _returnvalue
    (:Is%20Valid
      (Transformation|SetActorLocation _returnvalue Position false true))
    (:Is%20Not%20Valid
      (Development|PrintString "Invalid Player trying to Position"))))

(fn StringtoColor
  (params (String :type String))
  (switch string String
    (:Brown
      (LocalVariables|SetResult "NewEnumerator0"))
    (:Red
      (LocalVariables|SetResult "NewEnumerator1"))
    (:Blue
      (LocalVariables|SetResult "NewEnumerator2"))
    (:Green
      (LocalVariables|SetResult "NewEnumerator3"))
    (:Gray
      (LocalVariables|SetResult "NewEnumerator4")))
  (return (LocalVariables|GetResult)))

(fn Reset
  ;[1 1 1] Hide the player to avoid collision when spawning actors
  (Spawning|PositionPlayer (Variables|Spawning|GetPlayerHideLocation))
  ;[1 1 1] Update the game mode
  (Helper|SetGameMode)
  ;[1 1 1] Analyze the tile map and clear it after
  (TileMap|AnalyzeTileMap)
  (TileMap|ClearGameTileMapLayer)
  ;[1 1 1] Spawn the boxes and goals
  (Spawning|SpawnGameActors)
  ;[1 1 1] Position the player
  (Spawning|PositionPlayer (Variables|Spawning|GetPlayerStartLocation)))

(fn SetGameMode
  (bind _asbp_push_push_puzzle_2dgame_mode (Utilities|Casting|CastToBP_PushPushPuzzle2DGameMode (Game|GetGameMode)))
  (Variables|Default|SetGameMode _asbp_push_push_puzzle_2dgame_mode))

(fn GetTileUserDataString
  (params (TileMapLocation :type STR%20Tile%20Map%20Location%20Structure))
  (return (Utilities|String|ToString(Name) (Class|TileMapBlueprintLibrary|GetTileUserData (Class|PaperTileMapComponent|GetTile (Variables|Default|GetTileMap) (.x TileMapLocation) (.y TileMapLocation) (.layer TileMapLocation))))))