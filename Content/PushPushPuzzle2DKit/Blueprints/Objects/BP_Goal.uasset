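; BP_Goal is a colored goal tile in a 2D push-box puzzle that tracks whether a box of the matching color sits on it.
; Overlap on OccupiedCollision stores the entering BP_Box and sets Occupied if its color equals the goal's, then clears the flag when that box leaves.
; UpdateColor sets the goal's color and maps the enum to the corresponding sprite.
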(event OnComponentBeginOverlap(OccupiedCollision)
  (params (OverlappedComponent :type Primitive%20Component%20Object%20Reference) (OtherActor :type Actor%20Object%20Reference) (OtherComp :type Primitive%20Component%20Object%20Reference) (OtherBodyIndex :type Integer) (bFromSweep :type Boolean) (SweepResult :type Hit%20Result%20Structure%20%28by%20ref%29))
  ;[1 1 1] Wheter overlapping the a box, check color and mark as occupied. Save the box in a variable
  (bind _asbp_box (Utilities|Casting|CastToBP_Box OtherActor))
  (Variables|Default|SetOccupied (Utilities|Enum|Equal(Enum) (Variables|/Game/PushPushPuzzle2DKit/Blueprints/Objects/BP_Box.BP_Box_C|GetColor _asbp_box) (Variables|Default|GetColor)))
  (Variables|Default|SetOccupyingBox _asbp_box))

(event OnComponentEndOverlap(OccupiedCollision)
  (params (OverlappedComponent :type Primitive%20Component%20Object%20Reference) (OtherActor :type Actor%20Object%20Reference) (OtherComp :type Primitive%20Component%20Object%20Reference) (OtherBodyIndex :type Integer))
  ;[1 1 1] If the box is moved again, mark as not occupied
  (if (== OtherActor (Variables|Default|GetOccupyingBox))
    (Variables|Default|SetOccupied false)))

(fn ConstructionScript)

(fn UpdateColor
  (params (Color :type ENUM_Color%20Enum :default "NewEnumerator0"))
  ;[1 1 1] Convert enum value to sprite and set it
  (bind _output_get (Variables|Default|SetColor Color))
  (Rendering|Components|Sprite|SetSprite (Variables|Default|GetRenderComponent) (Utilities|Select :Index _output_get :NewEnumerator0 "/Game/PushPushPuzzle2DKit/Sprites/Goals/SP_GoalBrown.SP_GoalBrown" :NewEnumerator1 "/Game/PushPushPuzzle2DKit/Sprites/Goals/SP_GoalRed.SP_GoalRed" :NewEnumerator2 "/Game/PushPushPuzzle2DKit/Sprites/Goals/SP_GoalBlue.SP_GoalBlue" :NewEnumerator3 "/Game/PushPushPuzzle2DKit/Sprites/Goals/SP_GoalGreen.SP_GoalGreen" :NewEnumerator4 "/Game/PushPushPuzzle2DKit/Sprites/Goals/SP_GoalGrey.SP_GoalGrey")))