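; Player for a 2D Sokoban-style puzzle, moving tile by tile on the XZ plane and pushing boxes.
; Axis input sets the facing flipbook for the GameInstance's selected character, then line traces allow steps into empty or Coin tiles, or push Movable actors with free space behind.
; Moves are instant or eased via MoveComponentTo.
; Successful moves increment the GameMode's counter and lock input for a delay before checking level completion.
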(event Custom|Move
  (params (Direction :type ENUM_Direction%20Enum :default "NewEnumerator0"))
  ;[1 1 1] Check that can move is true and the game is not over
  (if (and (Variables|Movement|GetCanMove) (not (Variables|/Game/PushPushPuzzle2DKit/Blueprints/Game/BP_PushPushPuzzle2DGameMode.BP_PushPushPuzzle2DGameMode_C|GetLevelComplete (Variables|GameVariables|GetGameMode))))
    ;[1 1 1] Update animation direction and try to move
    (Animation|UpdateAnimation Direction)
    (bind _success (Movement|TryMove Direction))
    (if _success
      ;[1 1 1] If move was successful, increment number and start delay
      (Default|IncrementPlayerMoves (Variables|GameVariables|GetGameMode))
      (Variables|Movement|SetCanMove false)
      (Utilities|FlowControl|Delay (Variables|Movement|GetMoveDelayTime))
      ;[1 1 1] Check if the move finished the level and enable movement again
      (Default|CheckLevelComplete (Variables|GameVariables|GetGameMode))
      (Variables|Movement|SetCanMove true))))

(event Custom|LerpTo
  (params (HitActor :type Actor%20Object%20Reference) (MoveOffset :type Vector))
  ;[1 1 1] Check if we have a valid HitActor. If so, move that one first
  (if (Utilities|IsValid HitActor)
    (Utilities|FlowControl|Sequence
      (:then_0
        (Components|MoveComponentTo (Variables|/Script/Engine.Actor|GetRootComponent HitActor) (+ (Transformation|GetActorLocation HitActor) MoveOffset) "0, 0, 0" true true (Variables|Movement|GetLerpMoveTime) false))
      (:then_1
        ;[1 1 1] Always move the player
        (Components|MoveComponentTo (Variables|Transformation|GetRootComponent) (+ (Transformation|GetActorLocation) MoveOffset) "0, 0, 0" true true (Variables|Movement|GetLerpMoveTime) false :!label _label)))
    (else
      (goto _label))))

(event EventBeginPlay
  ;[1 1 1] Set variables
  (GameVariables|GetGameMode)
  (GameVariables|GetGameInstance)
  ;[1 1 1] Set initial animation
  (Animation|UpdateAnimation "NewEnumerator1"))

(event Input|AxisEvents|InputAxisMoveUp
  (params (AxisValue :type Float%20%28single-precision%29))
  ;[1 1 1] Check negative and positive threshold for moving down or up
  (if (<= AxisValue (Variables|Movement|GetMoveNegativeThreshold))
    (CallFunction|Move "NewEnumerator1")
    (elif (>= AxisValue (Variables|Movement|GetMovePositiveThreshold))
      (CallFunction|Move "NewEnumerator0"))))

(event Input|AxisEvents|InputAxisMoveRight
  (params (AxisValue :type Float%20%28single-precision%29))
  ;[1 1 1] Check negative and positive threshold for moving left or right
  (if (<= AxisValue (Variables|Movement|GetMoveNegativeThreshold))
    (CallFunction|Move "NewEnumerator3")
    (elif (>= AxisValue (Variables|Movement|GetMovePositiveThreshold))
      (CallFunction|Move "NewEnumerator2"))))

(fn ConstructionScript)

(fn DirectiontoVector
  (params (Direction :type ENUM_Direction%20Enum :default "NewEnumerator0") (TileSize :type Float%20%28single-precision%29))
  (return (* (Utilities|Select :Index Direction :NewEnumerator0 "0.000000, 0,1.000000" :NewEnumerator1 "0.000000,0.000000,-1.000000" :NewEnumerator2 "1.000000,0.000000,0.000000" :NewEnumerator3 "-1.000000, 0, 0") TileSize)))

(fn TryMove
  (params (Direction :type ENUM_Direction%20Enum :default "NewEnumerator0"))
  (bind _returnvalue (Transformation|GetActorLocation))
  ;[1 1 1] Calculate the move offset
  (LocalVariables|SetMoveOffset (Movement|DirectiontoVector Direction 128.0))
  ;[1 1 1] Check if the new position is occupied (hit by linetrace)
  (bind (_outhit _returnvalue_2) (Collision|LineTraceByChannel _returnvalue (+ _returnvalue (LocalVariables|GetMoveOffset)) "TraceTypeQuery1" false 0 "None"))
  (if _returnvalue_2
    (bind _output_get (LocalVariables|SetHitActor (.HitActor (Collision|BreakHitResult _outhit))))
    ;[1 1 1] Check if the object we hit is moveable (e.g. a box) or a coin. If not, the move was unsuccessful
    (if (Actor|ActorHasTag _output_get "Movable")
      ;[1 1 1] Check if the position behind the hit object is occupied (hit by linetrace)
      (bind _returnvalue_3 (Collision|LineTraceByChannel (Transformation|GetActorLocation (LocalVariables|GetHitActor)) (+ (Transformation|GetActorLocation (LocalVariables|GetHitActor)) (LocalVariables|GetMoveOffset)) "TraceTypeQuery1" false (Utilities|Array|MakeArray (LocalVariables|GetHitActor)) "None" false))
      (if _returnvalue_3
        ;[1 1 1] If the position behind the hit actor is occupied we cannot move it, so we cannot move the player
        (LocalVariables|SetMoveSuccessful false)
        (else
          (if (Variables|Movement|GetLerpMovement)
            ;[1 1 1] If the space is free, move the object and move the player after smoothly
            (CallFunction|Lerpto (LocalVariables|GetHitActor) (LocalVariables|GetMoveOffset))
            (else
              ;[1 1 1] If the space is free, move the object and move the player after instantly.
              (Transformation|AddActorWorldOffset (LocalVariables|GetHitActor) (LocalVariables|GetMoveOffset) true)
              (Transformation|AddActorWorldOffset (LocalVariables|GetMoveOffset) true)))
          ;[1 1 1] The move was successful
          (LocalVariables|SetMoveSuccessful true)))
      (elif (Actor|ActorHasTag _output_get "Coin")
        (if (Variables|Movement|GetLerpMovement) :!label _label
          ;[1 1 1] Lerp the movement (and possibly pick-up coin)
          (CallFunction|Lerpto 0 (LocalVariables|GetMoveOffset))
          (else
            ;[1 1 1] Instant move the player (and possibly pick-up coin)
            (Transformation|AddActorWorldOffset (LocalVariables|GetMoveOffset) true)))
        ;[1 1 1] mark the move as successful
        (LocalVariables|SetMoveSuccessful true)
        (else
          (LocalVariables|SetMoveSuccessful false))))
    (else
      (goto _label)))
  (return (LocalVariables|GetMoveSuccessful)))

(fn UpdateAnimation
  (params (Direction :type ENUM_Direction%20Enum :default "NewEnumerator0"))
  (Sprite|SetFlipbook (Variables|Default|GetSprite) (Animation|GetPlayerAnimation (Variables|/Game/PushPushPuzzle2DKit/Blueprints/Game/BP_PushPushPuzzle2DGameInstance.BP_PushPushPuzzle2DGameInstance_C|GetPlayerCharacter (Variables|GameVariables|GetGameInstance)) Direction)))

(fn GetPlayerAnimation
  (params (PlayerCharacter :type ENUM_PlayerCharacter%20Enum :default "NewEnumerator0") (Direction :type ENUM_Direction%20Enum :default "NewEnumerator0"))
  ;[1 1 1] Switch on selected character
  (switch Utilities|FlowControl|Switch|SwitchonENUM_PlayerCharacter PlayerCharacter
    (:NewEnumerator0
      (LocalVariables|SetResult (Utilities|Select :Index Direction :NewEnumerator0 "/Game/PushPushPuzzle2DKit/Animations/Plumber1/FB_Plumber1Up.FB_Plumber1Up" :NewEnumerator1 "/Game/PushPushPuzzle2DKit/Animations/Plumber1/FB_Plumber1Down.FB_Plumber1Down" :NewEnumerator2 "/Game/PushPushPuzzle2DKit/Animations/Plumber1/FB_Plumber1Right.FB_Plumber1Right" :NewEnumerator3 "/Game/PushPushPuzzle2DKit/Animations/Plumber1/FB_Plumber1Left.FB_Plumber1Left")))
    (:NewEnumerator2
      (LocalVariables|SetResult (Utilities|Select :Index Direction :NewEnumerator0 "/Game/PushPushPuzzle2DKit/Animations/Plumber2/FB_Plumber2Up.FB_Plumber2Up" :NewEnumerator1 "/Game/PushPushPuzzle2DKit/Animations/Plumber2/FB_Plumber2Down.FB_Plumber2Down" :NewEnumerator2 "/Game/PushPushPuzzle2DKit/Animations/Plumber2/FB_Plumber2Right.FB_Plumber2Right" :NewEnumerator3 "/Game/PushPushPuzzle2DKit/Animations/Plumber2/FB_Plumber2Left.FB_Plumber2Left")))
    (:NewEnumerator1
      (LocalVariables|SetResult (Utilities|Select :Index Direction :NewEnumerator0 "/Game/PushPushPuzzle2DKit/Animations/CoolGuy/FB_CoolGuyUp.FB_CoolGuyUp" :NewEnumerator1 "/Game/PushPushPuzzle2DKit/Animations/CoolGuy/FB_CoolGuyDown.FB_CoolGuyDown" :NewEnumerator2 "/Game/PushPushPuzzle2DKit/Animations/CoolGuy/FB_CoolGuyRight.FB_CoolGuyRight" :NewEnumerator3 "/Game/PushPushPuzzle2DKit/Animations/CoolGuy/FB_CoolGuyLeft.FB_CoolGuyLeft"))))
  (return (LocalVariables|GetResult)))

(fn GetGameMode
  ;[1 1 1] Get the GameMode
  (bind _asbp_push_push_puzzle_2dgame_mode (Utilities|Casting|CastToBP_PushPushPuzzle2DGameMode (Game|GetGameMode)))
  ;[1 1 1] Save in variable when Valid
  (Utilities|IsValid _asbp_push_push_puzzle_2dgame_mode
    (:Is%20Valid
      (Variables|GameVariables|SetGameMode _asbp_push_push_puzzle_2dgame_mode))))

(fn GetGameInstance
  ;[1 1 1] Get the GameInstance
  (bind _asbp_push_push_puzzle_2dgame_instance (Utilities|Casting|CastToBP_PushPushPuzzle2DGameInstance (Game|GetGameInstance)))
  ;[1 1 1] Save in variable when Valid
  (Utilities|IsValid _asbp_push_push_puzzle_2dgame_instance
    (:Is%20Valid
      (Variables|GameVariables|SetGameInstance _asbp_push_push_puzzle_2dgame_instance))))