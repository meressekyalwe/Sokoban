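; Game instance for the PushPushPuzzle2D kit that holds level data, the level to load and player progress across levels.
; On Init it snapshots the default level data for resets, then loads the save slot or creates a save object.
; Saved records merge into level data by ID, and SaveGame writes them back.
; Helpers unlock the next level, supply the current TileMap and keep best moves, time and coins, treating zero as unset.
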(event EventInit
  ;[1 1 1] Reset level data
  (Variables|Default|SetResetData (Variables|Default|GetLevelGameData))
  ;[1 1 1] Check if a save game exists
  (bind _returnvalue (SaveGame|DoesSaveGameExist (Variables|Default|GetSaveGameSlotName) (Variables|Default|GetSaveGameUserIndex)))
  (if _returnvalue
    ;[1 1 1] Load if it exists
    (CallFunction|LoadSaveGame)
    (else
      ;[1 1 1] Else create a save game and save it in a variable
      (Development|PrintString "No Save Game Found" true true "(R=1.000000,G=0.000000,B=0.000000,A=1.000000)")
      (bind _returnvalue_2 (SaveGame|CreateSaveGameObject "/Game/PushPushPuzzle2DKit/Blueprints/Game/BP_PushPushPuzzle2DSaveGame.BP_PushPushPuzzle2DSaveGame_C"))
      (Variables|Default|SetMySaveGame _returnvalue_2))))

(fn UnlockNextLevel
  ;[1 1 1] Get the current level index
  (if (.Exists (CallFunction|FindLevelGameData (Variables|Default|GetLevelToLoad)))
    ;[1 1 1] Increment the index and find the level
    (LocalVariables|SetLevelIndexToUnlock (+ (.Index (CallFunction|FindLevelGameData (Variables|Default|GetLevelToLoad))) 1))
    (if (Utilities|Array|IsValidIndex (Variables|Default|GetLevelGameData) (LocalVariables|GetLevelIndexToUnlock))
      ;[1 1 1] Unlock the level
      (Utilities|Struct|SetmembersinSTR_LevelGameData (Utilities|Array|Get(acopy) (Variables|Default|GetLevelGameData) (LocalVariables|GetLevelIndexToUnlock)) true)
      ;[1 1 1] Set the ID as the level to load next
      (Variables|Default|SetLevelToLoad (.ID (Utilities|Struct|BreakSTR_LevelGameData (Utilities|Array|Get(acopy) (Variables|Default|GetLevelGameData) (LocalVariables|GetLevelIndexToUnlock))))))
    (else
      (Development|PrintString "Trying to load non-existing level" true true "(R=1.000000,G=0.000000,B=0.000000,A=1.000000)"))))

(fn LoadSaveGame
  ;[1 1 1] Load the data from the file and set the Level Save Data
  (bind _returnvalue (SaveGame|LoadGamefromSlot (Variables|Default|GetSaveGameSlotName) (Variables|Default|GetSaveGameUserIndex)))
  (bind _asbp_push_push_puzzle_2dsave_game (Utilities|Casting|CastToBP_PushPushPuzzle2DSaveGame _returnvalue)
    (:then
      (bind _output_get (Variables|Default|SetMySaveGame _asbp_push_push_puzzle_2dsave_game))
      (Variables|Default|SetLevelSaveData (Variables|/Game/PushPushPuzzle2DKit/Blueprints/Game/BP_PushPushPuzzle2DSaveGame.BP_PushPushPuzzle2DSaveGame_C|GetLevelSaveDataValues _output_get))
      ;[1 1 1] Apply the save data to the level data
      (CallFunction|UpdateLevelDatawithSaveData (Variables|/Game/PushPushPuzzle2DKit/Blueprints/Game/BP_PushPushPuzzle2DSaveGame.BP_PushPushPuzzle2DSaveGame_C|GetLevelSaveDataValues _output_get)))
    (:CastFailed
      (Development|PrintString "Error: Save Game invalid Class" true true "(R=1.000000,G=0.000000,B=0.000000,A=1.000000)"))))

(fn ClearSaveGame
  ;[1 1 1] If the save game exists, delete it
  (bind _returnvalue (SaveGame|DoesSaveGameExist (Variables|Default|GetSaveGameSlotName) (Variables|Default|GetSaveGameUserIndex)))
  (if _returnvalue
    (SaveGame|DeleteGameinSlot (Variables|Default|GetSaveGameSlotName) (Variables|Default|GetSaveGameUserIndex)))
  ;[1 1 1] Clear SaveData
  (Utilities|Array|Clear (Variables|Default|GetLevelSaveData))
  ;[1 1 1] Clear Level Data
  (Utilities|Array|Clear (Variables|Default|GetLevelGameData))
  ;[1 1 1] Reset LevelData using Reset Data
  (Variables|Default|SetLevelGameData (Variables|Default|GetResetData)))

(fn SaveGame
  ;[1 1 1] Loop through the level game data
  (for _array_element (Variables|Default|GetLevelGameData)
    (if (.Exists (CallFunction|FindLevelSaveData (.id _array_element)))
      ;[1 1 1] Update existing Save Data
      (Utilities|Struct|SetmembersinSTR_LevelSaveData (Utilities|Array|Get(acopy) (Variables|Default|GetLevelSaveData) (.Index (CallFunction|FindLevelSaveData (.id _array_element)))) (.unlocked _array_element) (.leastmoves _array_element) (.besttime _array_element) (.mostcoins _array_element))
      (else
        ;[1 1 1] Add new Save Data
        (Utilities|Array|AddUnique (Variables|Default|GetLevelSaveData) (Utilities|Struct|MakeSTR_LevelSaveData (.id _array_element) (.unlocked _array_element) (.leastmoves _array_element) (.besttime _array_element) (.mostcoins _array_element))))))
  ;[1 1 1] Save the updated SaveLevelData to the file system
  (bind _mysavegame (Variables|Default|GetMySaveGame)
    (:then
      (Variables|/Game/PushPushPuzzle2DKit/Blueprints/Game/BP_PushPushPuzzle2DSaveGame.BP_PushPushPuzzle2DSaveGame_C|SetLevelSaveDataValues _mysavegame (Variables|Default|GetLevelSaveData))
      (bind _returnvalue (SaveGame|SaveGametoSlot (Variables|Default|GetMySaveGame) (Variables|Default|GetSaveGameSlotName) (Variables|Default|GetSaveGameUserIndex)))
      (if (not _returnvalue)
        (Development|PrintString "Save Unsuccessful" true true "(R=1.000000,G=0.000000,B=0.000000,A=1.000000)")))
    (:else
      (Development|PrintString "SaveGame Invalid" true true "(R=1.000000,G=0.000000,B=0.000000,A=1.000000)"))))

(fn FindLevelGameData
  (params (ID :type Guid%20Structure))
  ;[1 1 1] Loop through the level data
  (for (_array_element _array_index) (Variables|Default|GetLevelGameData)
    ;[1 1 1] If the level ID matches return the index, else -1
    (if (== (.id _array_element) ID)
      (LocalVariables|SetResult _array_index)
      (return (!= (LocalVariables|GetResult) -1) (LocalVariables|GetResult))))
  (return (!= (LocalVariables|GetResult) -1) (LocalVariables|GetResult)))

(fn GetCurrentTileMap
  (bind _leveltoload (Variables|Default|GetLevelToLoad))
  (bind (_exists _index) (CallFunction|FindLevelGameData _leveltoload))
  ;[1 1 1] Check if the level exists
  (if _exists
    (return (.tilemap (Utilities|Array|Get(acopy) (Variables|Default|GetLevelGameData) _index)))
    (else
      (Development|PrintString "Trying to get TileMap of Non-Existing Level" true true "(R=1.000000,G=0.000000,B=0.000000,A=1.000000)"))))

(fn FindLevelSaveData
  (params (ID :type Guid%20Structure))
  ;[1 1 1] Loop through the level data
  (for (_array_element _array_index) (Variables|Default|GetLevelSaveData)
    ;[1 1 1] If the level ID matches return the index, else -1
    (if (== (.id _array_element) ID)
      (LocalVariables|SetResult _array_index)
      (return (!= (LocalVariables|GetResult) -1) (LocalVariables|GetResult))))
  (return (!= (LocalVariables|GetResult) -1) (LocalVariables|GetResult)))

(fn UpdateLevelData
  (params (Moves :type Integer) (Time :type Float%20%28single-precision%29) (Coins :type Integer))
  (bind _levelgamedata (Variables|Default|GetLevelGameData))
  (bind _leveltoload (Variables|Default|GetLevelToLoad))
  (bind (_exists _index) (CallFunction|FindLevelGameData _leveltoload))
  (bind _output (Utilities|Array|Get(acopy) _levelgamedata _index))
  (bind (_id _hudbuttontext _tilemap _unlocked _leastmoves _besttime _mostcoins) (Utilities|Struct|BreakSTR_LevelGameData _output))
  (if _exists
    ;[1 1 1] Compare the moves, time, and coins, and set the new best moves, time and coins
    (bind (_mininteger _improved) (Compare|GetMinInteger _leastmoves Moves))
    (bind (_minfloat _improved_2) (Compare|GetMinFloat _besttime Time))
    (bind (_maxinteger _improved_3) (Compare|GetMaxInteger _mostcoins Coins))
    (Utilities|Struct|SetmembersinSTR_LevelGameData _output _mininteger _minfloat _maxinteger)
    (return _improved _improved_2 _improved_3)))

(fn UpdateLevelDatawithSaveData
  (params (SaveData :type Array%20of%20STR%20Level%20Save%20Data%20Structures))
  ;[1 1 1] Loop through the save data
  (for _array_element SaveData
    ;[1 1 1] Find the matching level data, and if it exists update the least moves and best time
    (if (.Exists (CallFunction|FindLevelGameData (.id _array_element)))
      (Utilities|Struct|SetmembersinSTR_LevelGameData (Utilities|Array|Get(acopy) (Variables|Default|GetLevelGameData) (.Index (CallFunction|FindLevelGameData (.id _array_element)))) (.unlocked _array_element) (.leastmoves _array_element) (.besttime _array_element) (.mostcoins _array_element)))))

(fn GetMinInteger
  (params (PreviousInteger :type Integer) (NewInteger :type Integer))
  (bind _returnvalue (== PreviousInteger 0))
  (bind _returnvalue_2 (< NewInteger PreviousInteger))
  (bind _returnvalue_3 (or _returnvalue _returnvalue_2))
  (return (select _returnvalue_3 NewInteger PreviousInteger) _returnvalue_3))

(fn GetMinFloat
  (params (PreviousFloat :type Float%20%28single-precision%29) (NewFloat :type Float%20%28single-precision%29))
  (bind _returnvalue (< NewFloat PreviousFloat))
  (bind _returnvalue_2 (== PreviousFloat 0.0))
  (bind _returnvalue_3 (or _returnvalue_2 _returnvalue))
  (return (select _returnvalue_3 NewFloat PreviousFloat) _returnvalue_3))

(fn HasSaveGame
  (bind _returnvalue (SaveGame|DoesSaveGameExist (Variables|Default|GetSaveGameSlotName) (Variables|Default|GetSaveGameUserIndex)))
  (return _returnvalue))

(fn GetMaxInteger
  (params (PreviousInteger :type Integer) (NewInteger :type Integer))
  (bind _returnvalue (== PreviousInteger 0))
  (bind _returnvalue_2 (!= NewInteger 0))
  (bind _returnvalue_3 (> NewInteger PreviousInteger))
  (bind _returnvalue_4 (and _returnvalue _returnvalue_2))
  (bind _returnvalue_5 (or _returnvalue_4 _returnvalue_3))
  (return (select _returnvalue_5 NewInteger PreviousInteger) _returnvalue_5))

(fn IsNextLevelAvailable
  (bind _leveltoload (Variables|Default|GetLevelToLoad))
  (bind (_exists _index) (CallFunction|FindLevelGameData _leveltoload))
  ;[1 1 1] Get the current level index
  (if _exists
    (return (Utilities|Array|IsValidIndex (Variables|Default|GetLevelGameData) (+ _index 1)))))