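; Game mode for the 2D push-box puzzle that runs each level, tracking moves, elapsed time, coins and goal completion.
; ResetMap, run at BeginPlay, destroys boxes, goals and coins, loads the current tile map from the game instance into the level actor and zeroes the stats.
; When all goals are occupied, it records results in the game instance, shows the completion overview via the player controller, unlocks the next level and saves.
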(event EventBeginPlay
  ;[1 1 1] Save the game instance
  (CallFunction|GetGameInstance)
  ;[1 1 1] Reset the map when game starts
  (CallFunction|ResetMap))

(fn ConstructionScript)

(fn CheckLevelComplete
  ;[1 1 1] Loop through the goals and check if they are occupied
  (bind _array_element (Utilities|Array|ForEachLoopwithBreak (Variables|Default|GetGoals) :!label _label)
    (:LoopBody
      (Utilities|IsValid _array_element
        (:Is%20Valid
          (if (not (Variables|/Game/PushPushPuzzle2DKit/Blueprints/Objects/BP_Goal.BP_Goal_C|GetOccupied _array_element))
            (LocalVariables|SetResult false)
            (goto _label Break)))))
    (:Completed
      (bind _output_get (Variables|Default|SetLevelComplete (LocalVariables|GetResult)))
      ;[1 1 1] If level is complete, call the function
      (if _output_get
        (CallFunction|OnLevelComplete)))))

(fn ResetMap
  ;[1 1 1] Clear the goals and mark as incomplete
  (Utilities|Array|Clear (Variables|Default|GetGoals))
  (Variables|Default|SetLevelComplete false)
  (Utilities|FlowControl|Sequence
    (:then_0
      ;[1 1 1] Destroy all boxes
      (bind _outactors (Actor|GetAllActorsOfClass "/Game/PushPushPuzzle2DKit/Blueprints/Objects/BP_Box.BP_Box_C"))
      (for _array_element _outactors
        (Utilities|IsValid _array_element
          (:Is%20Valid
            (Actor|DestroyActor _array_element)))))
    (:then_1
      ;[1 1 1] Destroy all goals
      (bind _outactors_2 (Actor|GetAllActorsOfClass "/Game/PushPushPuzzle2DKit/Blueprints/Objects/BP_Goal.BP_Goal_C"))
      (for _array_element_2 _outactors_2
        (Utilities|IsValid _array_element_2
          (:Is%20Valid
            (Actor|DestroyActor _array_element_2)))))
    (:then_2
      ;[1 1 1] Destroy all goals
      (bind _outactors_3 (Actor|GetAllActorsOfClass "/Game/PushPushPuzzle2DKit/Blueprints/Objects/BP_Coin.BP_Coin_C"))
      (for _array_element_3 _outactors_3
        (Utilities|IsValid _array_element_3
          (:Is%20Valid
            (Actor|DestroyActor _array_element_3)))))
    (:then_3
      ;[1 1 1] Reset the map
      (bind _outactors_4 (Actor|GetAllActorsOfClass "/Game/PushPushPuzzle2DKit/Blueprints/Level/BP_PushPushPuzzleLevel.BP_PushPushPuzzleLevel_C"))
      (Class|PaperTileMapComponent|SetTileMap (Variables|/Game/PushPushPuzzle2DKit/Blueprints/Level/BP_PushPushPuzzleLevel.BP_PushPushPuzzleLevel_C|GetTileMap (Utilities|Array|Get(acopy) _outactors_4)) (Default|GetCurrentTileMap (Variables|Default|GetGameInstance)))
      (Default|Reset (Utilities|Array|Get(acopy) _outactors_4)))
    (:then_4
      ;[1 1 1] Reset the player moves
      (Variables|Default|SetPlayerMoves 0))
    (:then_5
      ;[1 1 1] Reset the collected coins
      (Variables|Default|SetCoinsCollected 0))
    (:then_6
      ;[1 1 1] Set the start time to the current time
      (Variables|Default|SetStartTime (Utilities|Time|GetTimeSeconds)))))

(fn IncrementPlayerMoves
  (Variables|Default|SetPlayerMoves (+ (Variables|Default|GetPlayerMoves) 1)))

(fn OnLevelComplete
  (bind _returnvalue (Utilities|Time|GetTimeSeconds))
  (bind _coinscollected (Variables|Default|GetCoinsCollected))
  (bind _playermoves (Variables|Default|GetPlayerMoves))
  (bind _starttime (Variables|Default|GetStartTime))
  (bind _returnvalue_2 (- _returnvalue _starttime))
  ;[1 1 1] Update the level data
  (bind (_improvedmoves _improvedtime _improvedcoins) (Default|UpdateLevelData (Variables|Default|GetGameInstance) _playermoves _returnvalue_2 _coinscollected))
  ;[1 1 1] Show level complete overview to player
  (bind _asbp_push_push_puzzle_2dplayer_controller (Utilities|Casting|CastToBP_PushPushPuzzle2DPlayerController (Game|GetPlayerController 0)))
  (Default|ShowLevelCompleteOverview _asbp_push_push_puzzle_2dplayer_controller _playermoves _returnvalue_2 _coinscollected _improvedmoves _improvedtime _improvedcoins (Default|IsNextLevelAvailable (Variables|Default|GetGameInstance)))
  ;[1 1 1] Unlock next level
  (Default|UnlockNextLevel (Variables|Default|GetGameInstance))
  ;[1 1 1] Save the game
  (Default|SaveGame (Variables|Default|GetGameInstance)))

(fn GetGameInstance
  ;[1 1 1] Get the GameInstance
  (bind _asbp_push_push_puzzle_2dgame_instance (Utilities|Casting|CastToBP_PushPushPuzzle2DGameInstance (Game|GetGameInstance)))
  ;[1 1 1] Save in variable when Valid
  (Utilities|IsValid _asbp_push_push_puzzle_2dgame_instance
    (:Is%20Valid
      (Variables|Default|SetGameInstance _asbp_push_push_puzzle_2dgame_instance))))

(fn IncrementCollectedCoins
  (Variables|Default|SetCoinsCollected (+ (Variables|Default|GetCoinsCollected) 1)))